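; BP_Weapon_AR4 is the AR4 weapon Blueprint, which tracks its ammo count.
; Its construction script calls the parent's, then sets the starting and maximum ammo.
; Each Fire press handled by the weapon itself spends one round while ammo remains.
; When the last round is spent, it switches player 0's BP_SwatCharacter from firing to reloading through state flags, without refilling ammo here.
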(event Input|ActionEvents|InputActionFire
  (params (Key :type Key%20Structure :default "None"))
  (bind _returnvalue (Game|GetPlayerCharacter 0))
  (bind _asbp_swat_character (Utilities|Casting|CastToBP_SwatCharacter _returnvalue))
  (:Pressed
    (if (> (Variables|Default|GetAmmoCount) 0)
      (bind _result (Math|Integer|DecrementInt (Variables|Default|GetAmmoCount))
        (:%20%20
          (if (<= _result 0)
            (Variables|/Game/Character/Blueprints/BP_SwatCharacter.BP_SwatCharacter_C|SetIsFiring _asbp_swat_character false)
            (Variables|/Game/Character/Blueprints/BP_SwatCharacter.BP_SwatCharacter_C|SetIsReloading _asbp_swat_character true)))))))

(fn ConstructionScript
  (|CallParentFunction)
  (Variables|Default|SetAmmoCount 35)
  (Variables|Default|SetMaxAmmo 50))